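; BP_GameInstanceTest is a game instance Blueprint that holds shared enemy spawning state and a kill count.
; AddSpawner adds to a Spawners list, and RemoveEnemy increments Kills while decrementing EnemyCount.
; CanSpawn returns true only when DoSpawn is set and EnemyCount is below EnemyMaxCount.
; Nothing in these graphs increments EnemyCount or performs the spawning itself.
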(event `Add Spawner`
  (params (Spawners :type "/Game/Blueprints/BP_SpawnerTest Object Reference"))
  (`KismetArrayLibrary.Array_Add` (`self.Spawners`) Spawners))

(event `Remove Enemy`
  (`/Engine/EditorBlueprintResources/StandardMacros.IncrementInt` (`self.Kills`)
    (:`  `
      (`/Engine/EditorBlueprintResources/StandardMacros.DecrementInt` (`self.EnemyCount`)))))

(fn `CanSpawn`
  (returns (CanSpawn :type Boolean))
  (if (`self.DoSpawn`)
    (if (< (`self.EnemyCount`) (`self.EnemyMaxCount`))
      (return true)
      (else
        _)))
  (return false))