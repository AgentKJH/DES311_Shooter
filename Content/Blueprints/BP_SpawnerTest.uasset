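; BP_SpawnerTest is an enemy spawner actor that periodically creates BP_EnemyTest instances at its SpawnPoint transform.
; On BeginPlay it registers itself with BP_GameInstanceTest, then loops on a fixed delay, asking the game instance whether spawning is allowed.
; Each spawn increments the game instance's shared enemy count, so the game instance governs spawning centrally.
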(event `self.ReceiveBeginPlay`
  (bind _asbp_game_instance_test (cast `/Game/Blueprints/BP_GameInstanceTest` (`GameplayStatics.GetGameInstance`)))
  (bind _output_get (set `self.As BP Game Instance Test` _asbp_game_instance_test))
  (`/Game/Blueprints/BP_GameInstanceTest.Add Spawner` _output_get self)
  (bind _canspawn (`/Game/Blueprints/BP_GameInstanceTest.CanSpawn` (`self.As BP Game Instance Test`) :!label _label))
  (if _canspawn
    (`self.Spawn Enemy`))
  (`KismetSystemLibrary.Delay` 10.0)
  (goto _label))

(event `Spawn Enemy`
  (`/Engine/EditorBlueprintResources/StandardMacros.IncrementInt` (`/Game/Blueprints/BP_GameInstanceTest.EnemyCount` (`self.As BP Game Instance Test`))
    (:`  `
      (`|SpawnActorFromClass` "/Game/Blueprints/BP_EnemyTest.BP_EnemyTest_C" (`SceneComponent.K2_GetComponentToWorld` (`self.SpawnPoint`)) "Undefined" "MultiplyWithRoot" null null))))

(fn `UserConstructionScript`)