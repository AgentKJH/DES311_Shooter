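; BP_EnemyTest is a melee enemy that chases the player and can be shot dead.
; Tick starts a delayed AI MoveTo; on arrival, Attack sets an AnimBP flag and times a forward sphere trace to deal damage.
; Point damage spawns blood, with head-hitbox hits multiplied.
; Death ragdolls the mesh with a shot impulse, calls RemoveEnemy on the game instance, then destroys the actor after a delay.
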(event `Attack`
  (bind _capsulecomponent (`self.CapsuleComponent`))
  (bind _returnvalue (`SceneComponent.K2_GetComponentLocation` _capsulecomponent))
  (bind _asthird_person_anim_bp (cast `/Game/Assets/PolygonFantasyRivals/EpicContent/Mannequin/Animations/ThirdPerson_AnimBP` (`SkeletalMeshComponent.GetAnimInstance` (`self.Mesh`))))
  (set `/Game/Assets/PolygonFantasyRivals/EpicContent/Mannequin/Animations/ThirdPerson_AnimBP.Attacking` true _asthird_person_anim_bp)
  (`KismetSystemLibrary.Delay` 1.0)
  (bind _outhit (`KismetSystemLibrary.SphereTraceSingle` _returnvalue (+ _returnvalue (* (`SceneComponent.GetForwardVector` _capsulecomponent) (`self.AttackRange`))) 60.0 "TraceTypeQuery5"))
  (`GameplayStatics.ApplyDamage` (`.HitActor` (`GameplayStatics.BreakHitResult` _outhit)) (`self.Base Damage`) (`self.GetController`) null "/Script/Engine.DamageType")
  (`KismetSystemLibrary.Delay` 1.6)
  (set `/Game/Assets/PolygonFantasyRivals/EpicContent/Mannequin/Animations/ThirdPerson_AnimBP.Attacking` false _asthird_person_anim_bp)
  (set `self.ChasingPlayer` false))

(event `self.ReceiveTick`
  (params (DeltaSeconds :type "Float (single-precision)"))
  ;[0.05729 0.05729 0.05729] Call Chase
  (if (not (`self.ChasingPlayer`))
    (`KismetSystemLibrary.Delay` (`self.ChasePlayerDelay`))
    (set `self.ChasingPlayer` true)
    (`self.ChasePlayer`)))

(event `ChasePlayer`
  ;[0.05729 0.05729 0.05729] Chase Player
  (if (`self.DoChasePlayer`)
    (`|AIMoveTo` self (0.0 0.0 0.0) (`GameplayStatics.GetPlayerCharacter` 0) 100.0
      (:`OnSuccess`
        (`self.Attack`))
      (:`OnFail`
        (set `self.ChasingPlayer` false)))))

(event `self.ReceiveBeginPlay`
  ;[0.05729 0.05729 0.05729] Setup
  (add `self.OnTakePointDamage` (delegate `OnTakePointDamage_Event`))
  (bind _asbp_first_person_character (cast `/Game/FirstPerson/Blueprints/BP_FirstPersonCharacter` (`GameplayStatics.GetPlayerCharacter` 0)))
  (set `self.As BP First Person Character` _asbp_first_person_character)
  (`self.EnableInput` (`GameplayStatics.GetPlayerController` 0)))

(event `OnTakePointDamage_Event` :!signature `self.OnTakePointDamage`
  (params (DamagedActor :type "Actor Object Reference") (Damage :type "Float (single-precision)") (InstigatedBy :type "Controller Object Reference") (HitLocation :type "Vector Structure") (FHitComponent :type "PrimitiveComponent Object Reference") (BoneName :type Name) (ShotFromDirection :type "Vector Structure") (DamageType :type "DamageType Object Reference") (DamageCauser :type "Actor Object Reference"))
  ;[0.05729 0.05729 0.05729] Damage
  (`GameplayStatics.SpawnEmitterAtLocation` "/Game/Assets/PolygonFantasyRivals/Particles/FX_Blood.FX_Blood" HitLocation (struct) (3.0 3.0 3.0))
  (if (not (`self.Dead`))
    (if (== FHitComponent (`self.HeadHitBox`))
      (bind _die (`self.TakeDamage` (* Damage (`self.CritMultiplier`))))
      (if _die
        (set `self.Dead` true :!label _label)
        ;[0.05729 0.05729 0.05729] Death
        (`PrimitiveComponent.SetSimulatePhysics` (`self.Mesh`) true)
        (`PrimitiveComponent.SetCollisionEnabled` (`self.CapsuleComponent`) "NoCollision")
        (`PrimitiveComponent.AddImpulseAtLocation` (`self.Mesh`) (* ShotFromDirection 100000) HitLocation BoneName :!label _label_2)
        (`/Engine/EditorBlueprintResources/StandardMacros.DoOnce` false
          (:`Completed`
            ;[0.05729 0.05729 0.05729] Remove Refs and Destroy Actor
            (bind _asbp_game_instance_test (cast `/Game/Blueprints/BP_GameInstanceTest` (`GameplayStatics.GetGameInstance`)))
            (`/Game/Blueprints/BP_GameInstanceTest.Remove Enemy` _asbp_game_instance_test)
            (`KismetSystemLibrary.Delay` 3.0)
            (`self.K2_DestroyActor`))))
      (else
        (bind _die_2 (`self.TakeDamage` Damage))
        (if _die_2
          (goto _label))))
    (else
      (goto _label_2))))

(fn `TakeDamage`
  (params (Damage :type "Float (double-precision)"))
  (returns (Die :type Boolean))
  (bind _returnvalue (- (`self.Health`) Damage))
  (if (<= _returnvalue 0.0)
    (set `self.Health` _returnvalue)
    (return true)
    (else
      (set `self.Health` _returnvalue)
      (return false))))

(fn `UserConstructionScript`)